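; BP_HLOD is an actor that builds and animates a ring of Hierarchical Instanced Static Mesh instances around itself.
; BeginPlay places the instances on a circle using sine and cosine of the loop index, turning each toward the center with a fixed rotation offset.
; Tick adds a time-based sine offset to every instance's current Z, bobbing the ring in unison with frame-rate-dependent amplitude.
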(event EventBeginPlay
  (for _index (range 0 100)
    (Components|InstancedStaticMesh|AddInstance (Variables|Default|GetHierarchicalInstancedStaticMesh) (Math|Transform|MakeTransform (Math|Vector|MakeVector (* (Math|Trig|Cos(Radians) (Math|Conversions|ToFloat(Integer) _index)) 7.5e+02) (* (Math|Trig|Sin(Radians) (Math|Conversions|ToFloat(Integer) _index)) 7.5e+02) 0.0) (Math|Rotator|CombineRotators (Math|Rotator|FindLookatRotation (+ (Transformation|GetActorLocation) (Math|Vector|MakeVector (* (Math|Trig|Cos(Radians) (Math|Conversions|ToFloat(Integer) _index)) 7.5e+02) (* (Math|Trig|Sin(Radians) (Math|Conversions|ToFloat(Integer) _index)) 7.5e+02) 0.0)) (Transformation|GetActorLocation)) "0,-90.000000, 0")) false)))

(event EventTick
  (params (DeltaSeconds :type Float%20%28single-precision%29))
  (bind _hierarchicalinstancedstaticmesh (Variables|Default|GetHierarchicalInstancedStaticMesh))
  (for _index (range 0 100)
    (Components|InstancedStaticMesh|UpdateInstanceTransform _hierarchicalinstancedstaticmesh _index (Math|Transform|MakeTransform (+ (.location (.OutInstanceTransform (Components|InstancedStaticMesh|GetInstanceTransform _hierarchicalinstancedstaticmesh _index false))) (Math|Vector|MakeVector 0.0 0.0 (* (Math|Trig|Sin(Radians) (* (Utilities|Time|GetTimeSeconds) 5.0)) 2.0))) (.rotation (.OutInstanceTransform (Components|InstancedStaticMesh|GetInstanceTransform _hierarchicalinstancedstaticmesh _index false))) "1.000000,1.000000,1.000000") false false false)))

(fn ConstructionScript)